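; Player-controlled knight with four-direction Paper2D flipbook animation for idle and movement.
; Each tick polls the move axes, updates the animation, then sets Direction for the next update, with sideways input overriding vertical.
; Left reuses the side flipbook with the sprite rotated 180 degrees.
; BeginPlay adds the Enhanced Input mapping context; the attack action only toggles an Attack flag, and no movement is applied here.
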(event Input|EnhancedActionEvents|EnhancedInputActionIA_Attack
  (params (ActionValue :type Boolean) (ElapsedSeconds :type Float%20%28double-precision%29) (TriggeredSeconds :type Float%20%28double-precision%29) (InputAction :type Input%20Action%20Object%20Reference :default "/Game/Blueprints/IA_Attack.IA_Attack"))
  ;[0.15 0.15 0.15 0.5] 공격 인풋 액션 작동
  (:Started
    (Variables|Default|SetbAttack true))
  (:Canceled
    (Variables|Default|SetbAttack false)))

(event EventBeginPlay
  ;[0.15 0.15 0.15 0.5] 공격 인풋 액션 초기화
  (bind _as플레이어_컨트롤러 (Utilities|Casting|CastToPlayerController (Pawn|GetController)))
  (Input|AddMappingContext (PlayerController|LocalPlayerSubsystems|GetEnhancedInputLocalPlayerSubsystem _as플레이어_컨트롤러) "/Game/Blueprints/IMC_default.IMC_default" 0 "(bIgnoreAllPressedKeysUntilRelease=True,bForceImmediately=False,bNotifyUserSettings=False)"))

(event EventTick
  (params (DeltaSeconds :type Float%20%28single-precision%29))
  ;[0.15 0.15 0.15 0.5] 입력 함수 작동
  (CallFunction|UpdateInput))

(fn ConstructionScript)

(fn UpdateAnimation
  ;[0.15 0.15 0.15 0.5] 만약 키를 누르면 Idle, 안눌렀으면 Move 애니메이션
  (if (Variables|Default|GetbKeyboardPressed)
    (CallFunction|MoveAnimations)
    (else
      (CallFunction|IdleAnimations))))

(fn IdleAnimations
  (bind _sprite (Variables|Default|GetSprite))
  (switch Utilities|FlowControl|Switch|SwitchonEDirection (Variables|Default|GetDirection)
    (:NewEnumerator1
      (Sprite|SetFlipbook _sprite "/Game/Sprite/knight/up_idle.up_idle")
      (Transformation|SetRelativeRotation _sprite "0, 0, 0" false false :!label _label))
    (:NewEnumerator2
      (Sprite|SetFlipbook _sprite "/Game/Sprite/knight/down_idle.down_idle")
      (goto _label))
    (:NewEnumerator3
      (Sprite|SetFlipbook _sprite "/Game/Sprite/knight/side_idle.side_idle")
      (Transformation|SetRelativeRotation _sprite "0.000000,180.000000,0.000000" false false))
    (:NewEnumerator4
      (Sprite|SetFlipbook _sprite "/Game/Sprite/knight/side_idle.side_idle")
      (goto _label))))

(fn MoveAnimations
  (bind _sprite (Variables|Default|GetSprite))
  (switch Utilities|FlowControl|Switch|SwitchonEDirection (Variables|Default|GetDirection)
    (:NewEnumerator1
      (Sprite|SetFlipbook _sprite "/Game/Sprite/knight/up_move.up_move")
      (Transformation|SetRelativeRotation _sprite "0, 0, 0" false false :!label _label))
    (:NewEnumerator2
      (Sprite|SetFlipbook _sprite "/Game/Sprite/knight/down_move.down_move")
      (goto _label))
    (:NewEnumerator3
      (Sprite|SetFlipbook _sprite "/Game/Sprite/knight/side_move.side_move")
      (Transformation|SetRelativeRotation _sprite "0.000000,180.000000,0.000000" false false))
    (:NewEnumerator4
      (Sprite|SetFlipbook _sprite "/Game/Sprite/knight/side_move.side_move")
      (goto _label))))

(fn UpdateInput
  ;[0.15 0.15 0.15 0.5] wasd 입력 판단 및 애니메이션 실행
  (Utilities|FlowControl|Sequence
    (:then_0
      (Variables|Default|SetbKeyboardPressed (or (!= (Input|AxisValues|GetMoveUpDown) 0.0) (!= (Input|AxisValues|GetMoveSide) 0.0)))
      (CallFunction|UpdateAnimation))
    (:then_1
      ;[0.15 0.15 0.15 0.5] 어떤 키를 눌렀는지 구분하고 디렉션값 변경
      (Math|Float|CompareFloat (Input|AxisValues|GetMoveUpDown) 0.0
        (:>
          (Variables|Default|SetDirection "NewEnumerator1"))
        (:<
          (Variables|Default|SetDirection "NewEnumerator2"))))
    (:then_2
      (Math|Float|CompareFloat (Input|AxisValues|GetMoveSide) 0.0
        (:>
          (Variables|Default|SetDirection "NewEnumerator4"))
        (:<
          (Variables|Default|SetDirection "NewEnumerator3"))))))